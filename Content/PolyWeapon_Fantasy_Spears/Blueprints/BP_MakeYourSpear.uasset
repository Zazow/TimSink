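; BP_MakeYourSpear is an actor Blueprint that assembles a modular spear from three static mesh components: head, handle and counterweight.
; Its construction script assigns the chosen mesh variant to each component, then applies one shared SwordMaterial to material slot 0 of all three.
; The event graph holds no active logic, so the Blueprint only handles visual assembly.
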(event EventBeginPlay)

(event Collision|EventActorBeginOverlap
  (params (OtherActor :type Actor%20Object%20Reference)))

(event EventTick
  (params (DeltaSeconds :type Float%20%28single-precision%29)))

(fn ConstructionScript
  ;[1 1 1] Install static meshes
  (Components|StaticMesh|SetStaticMesh (Variables|Default|GetHeadMesh) (Variables|Default|GetHead))
  (Components|StaticMesh|SetStaticMesh (Variables|Default|GetСounterweight) (Variables|Default|GetСounterweight_Variant))
  (Components|StaticMesh|SetStaticMesh (Variables|Default|GetHandle) (Variables|Default|GetHandleVariant))
  ;[1 1 1] Material Assignment
  (Rendering|Material|SetMaterial (Variables|Default|GetСounterweight) 0 (Variables|Default|GetSwordMaterial)))